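; BP_Key is a maze key pickup that records its key number on the maze game mode when interacted with.
; BeginPlay caches the GM_Maze game mode, and Interact overwrites its Key value, prints the key's name with an acquired message, then destroys the actor.
; The construction script sets the sphere's material from KeyNumber, so the two handled key types look different in the editor.
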(event EventBeginPlay
  (bind _asgm_maze (Utilities|Casting|CastToGM_Maze (Game|GetGameMode)))
  (Variables|Default|SetAs%20GM%20Maze _asgm_maze))

(event EventInteract
  (bind _output_get (Variables|/Game/Labs/Common/GM_Maze.GM_Maze_C|SetKey (Variables|Default|GetAs%20GM%20Maze) (Variables|Default|GetKeyNumber)))
  (Development|PrintString (Utilities|String|Append (Utilities|Array|Get(acopy) (Variables|Default|GetNames) _output_get) " Key Acquired"))
  (Actor|DestroyActor))

(fn ConstructionScript
  (bind _sphere (Variables|Default|GetSphere))
  (switch int (Variables|Default|GetKeyNumber)
    (:0
      (Rendering|Material|SetMaterial _sphere 0 "/Engine/MapTemplates/Materials/BasicAsset03.BasicAsset03"))
    (:1
      (Rendering|Material|SetMaterial _sphere 0 "/Engine/MapTemplates/Materials/BasicAsset01.BasicAsset01"))))