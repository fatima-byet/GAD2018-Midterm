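; BP_Switch is an interactable switch that triggers traps of a chosen TrapType through the player character.
; On BeginPlay it caches the player as BP_ThirdPersonCharacter.
; Its Interact event passes TrapType to that character's CallDPTrap, so the switch holds no direct trap references.
; The construction script shows the TrapType enum name on its text component.
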(event EventBeginPlay
  (bind _asbp_third_person_character (Utilities|Casting|CastToBP_ThirdPersonCharacter (Game|GetPlayerCharacter 0)))
  (Variables|Default|SetPlayer _asbp_third_person_character))

(event EventInteract
  (Default|CallDPTrap (Variables|Default|GetPlayer) (Variables|Default|GetTrapType)))

(fn ConstructionScript
  (Rendering|Components|TextRender|SetText (Variables|Default|GetText) (Utilities|Text|ToText(String) (Utilities|String|EnumtoString (Variables|Default|GetTrapType)))))