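; Maze gate actor that shifts between two positions each time BP_ThirdPersonCharacter overlaps it.
; A FlipFlop alternates on each overlap, and its state is passed to the character through CallDPMazeGate.
; After a very short delay, the whole actor jumps by the EndLocation local offset or its inverse, with no sweep or interpolation.
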(event EventBeginPlay)

(event Collision|EventActorBeginOverlap
  (params (OtherActor :type Actor%20Object%20Reference))
  (bind _endlocation (Variables|Default|GetEndLocation))
  (bind _asbp_third_person_character (Utilities|Casting|CastToBP_ThirdPersonCharacter OtherActor))
  (bind _output_get (Variables|Default|SetAs%20BP%20Third%20Person%20Character _asbp_third_person_character))
  (bind _isa (Utilities|FlowControl|FlipFlop)
    (:A
      _)
    (:B
      _))
  (Default|CallDPMazeGate _output_get _isa)
  (if _isa
    (Utilities|FlowControl|Delay 0.02)
    (Transformation|AddActorLocalOffset _endlocation false false)
    (else
      (Utilities|FlowControl|Delay 0.02)
      (Transformation|AddActorLocalOffset (* _endlocation -1.0) false false))))

(event EventTick
  (params (DeltaSeconds :type Float%20%28single-precision%29)))

(fn ConstructionScript)