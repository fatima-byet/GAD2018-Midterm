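; Interactable door Blueprint that swings open and closed each time it receives Interact.
; Interact flips the InteractState flag and plays or reverses DoorTimeline, whose rotation track lerps the Door component's relative rotation through a 90-degree turn.
; GetInteractState exposes the current state to callers.
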(event EventBeginPlay)

(event Collision|EventActorBeginOverlap
  (params (OtherActor :type Actor%20Object%20Reference)))

(event EventTick
  (params (DeltaSeconds :type Float%20%28single-precision%29)))

(event EventInteract
  (if (Variables|Default|GetInteract%20State)
    (Variables|Default|SetInteract%20State false)
    (bind _doorrotationtrack (Timeline|DoorTimeline Reverse)
      (:Update
        (Transformation|SetRelativeRotation (Variables|Default|GetDoor) (Math|Rotator|Lerp(Rotator) "0, 0, 0" "0.000000,-90.000000,0.000000" _doorrotationtrack) false false)))
    (else
      (Variables|Default|SetInteract%20State true)
      (Timeline|DoorTimeline Play))))

(fn ConstructionScript)

(fn GetInteractState
  (return (Variables|Default|GetInteract%20State)))