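; BP_DispatcherLight is an event dispatcher example: a point light that changes color when the player character is hit.
; On BeginPlay it caches the BP_ThirdPersonCharacter and binds to its DPGotHit dispatcher, randomizing the light's RGB on each broadcast and ignoring the Health payload.
; When that character overlaps the Box, it unbinds all listeners from the dispatcher, not just this light; a single-event unbind node is left unconnected.
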(event OnComponentBeginOverlap(Box)
  (params (OverlappedComponent :type Primitive%20Component%20Object%20Reference) (OtherActor :type Actor%20Object%20Reference) (OtherComp :type Primitive%20Component%20Object%20Reference) (OtherBodyIndex :type Integer) (bFromSweep :type Boolean) (SweepResult :type Hit%20Result%20Structure%20%28by%20ref%29))
  (if (== OtherActor (Variables|Default|GetAs%20BP%20Third%20Person%20Character))
    (EventDispatchers|UnbindallEventsfromDPGotHit (Variables|Default|GetAs%20BP%20Third%20Person%20Character))))

(event Custom|DP_GotHit_Event
  (params (Health :type Float%20%28double-precision%29))
  (Rendering|Components|Light|SetLightColor (Variables|Default|GetPointLight) (Utilities|Struct|MakeLinearColor (Math|Random|RandomFloat) (Math|Random|RandomFloat) (Math|Random|RandomFloat) 1.0) true))

(event EventBeginPlay
  (bind _asbp_third_person_character (Utilities|Casting|CastToBP_ThirdPersonCharacter (Game|GetPlayerCharacter 0)))
  (bind _output_get (Variables|Default|SetAs%20BP%20Third%20Person%20Character _asbp_third_person_character))
  (EventDispatchers|AssignDPGotHit _output_get (delegate Custom|DP_GotHit_Event)))

(fn ConstructionScript)