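; BP_Door is a keyed door for the maze lab that slides open on Interact when the key held in GM_Maze matches its DoorKey.
; A timeline lerps the door component's relative location from the origin to EndLocation; a mismatched key prints an on-screen warning instead.
; The construction script picks the door's material from DoorKey, visually distinguishing the two handled key types.
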(event EventBeginPlay
  (bind _asgm_maze (Utilities|Casting|CastToGM_Maze (Game|GetGameMode)))
  (Variables|Default|SetAs%20GM%20Maze _asgm_maze))

(event EventInteract
  (if (== (Variables|Default|GetDoorKey) (Variables|/Game/Labs/Common/GM_Maze.GM_Maze_C|GetKey (Variables|Default|GetAs%20GM%20Maze)))
    (bind _newtrack_0 (Timeline|DoorTimeline Play)
      (:Update
        (Transformation|SetRelativeLocation (Variables|Default|GetDoor) (Math|Vector|Lerp(Vector) "0, 0, 0" (Variables|Default|GetEndLocation) _newtrack_0) false false)))
    (else
      (Development|PrintString "YOU DONT HAVE THE CORRECT KEY!" true true "(R=1.000000,G=0.038433,B=0.000000,A=1.000000)"))))

(fn ConstructionScript
  (bind _door (Variables|Default|GetDoor))
  (switch int (Variables|Default|GetDoorKey)
    (:0
      (Rendering|Material|SetMaterial _door 0 "/Engine/MapTemplates/Materials/BasicAsset03.BasicAsset03"))
    (:1
      (Rendering|Material|SetMaterial _door 0 "/Engine/MapTemplates/Materials/BasicAsset01.BasicAsset01"))))