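; BP_Gold is an interactable gold pickup for the maze game mode, worth a random amount of gold.
; The construction script rolls the value and calls a CreateMesh macro against descending thresholds, so richer pickups show more meshes.
; Each mesh gets a random offset, yaw and scale for a scattered pile look.
; Interact adds the value to GM_Maze's CurrentGold, prints the new total and destroys the actor.
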(event EventBeginPlay
  (bind _asgm_maze (Utilities|Casting|CastToGM_Maze (Game|GetGameMode)))
  (Variables|Default|SetAs%20GM%20Maze _asgm_maze))

(event EventInteract
  (bind _as_gm_maze (Variables|Default|GetAs%20GM%20Maze))
  (bind _output_get (Variables|/Game/Labs/Common/GM_Maze.GM_Maze_C|SetCurrentGold _as_gm_maze (+ (Variables|/Game/Labs/Common/GM_Maze.GM_Maze_C|GetCurrentGold _as_gm_maze) (Variables|Default|GetGold))))
  (Development|PrintString (Utilities|String|ToString(Integer) _output_get) true true "(R=1.000000,G=0.489296,B=0.000000,A=1.000000)")
  (Actor|DestroyActor))

(fn ConstructionScript
  (Variables|Default|SetGold (Math|Random|RandomIntegerinRange 1 99))
  (Utilities|CreateMesh (>= (Variables|Default|GetGold) 76)
    (:Output
      _)
    (:False
      _))
  (Utilities|CreateMesh (>= (Variables|Default|GetGold) 26)
    (:Output
      _)
    (:False
      _))
  (Utilities|CreateMesh (>= (Variables|Default|GetGold) 1)))