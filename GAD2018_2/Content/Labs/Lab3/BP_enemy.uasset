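; BP_enemy is an enemy pawn that starts chasing the player once it spots a pawn.
; PawnSensing's see-pawn event sets IsSeeingPlayer, which is never cleared here, and calls FollowPlayer.
; FollowPlayer uses AI MoveTo toward the player character and prints a debug message.
; BeginPlay caches the player as BP_ThirdPersonCharacter, though the chase fetches the player character directly.
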(event OnSeePawn(PawnSensing)
  (params (Pawn :type Pawn%20Object%20Reference))
  (Variables|Default|SetisSeeingPlayer true)
  (CallFunction|FollowPlayer))

(event Custom|FollowPlayer
  (if (Variables|Default|GetisSeeingPlayer)
    (AI|AIMoveTo self "0, 0, 0" (Game|GetPlayerCharacter 0) 2e+01 false
      (:then
        (Development|PrintString "help this person escape")))))

(event EventBeginPlay
  (bind _asbp_third_person_character (Utilities|Casting|CastToBP_ThirdPersonCharacter (Game|GetPlayerCharacter 0)))
  (Variables|Default|SetPlayer _asbp_third_person_character))

(event Collision|EventActorBeginOverlap
  (params (OtherActor :type Actor%20Object%20Reference)))

(event EventTick
  (params (DeltaSeconds :type Float%20%28single-precision%29)))

(fn ConstructionScript)