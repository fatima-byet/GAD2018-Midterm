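; BP_MazeCell is one modular maze tile that can hold a spike, axe or gas trap.
; The construction script builds floor, optional walls, ceiling and spotlight from grid size, and sets the trap as a child actor.
; On BeginPlay, trapless cells may randomly spawn a medkit or gold in that slot.
; It binds an event to the player's maze-gate dispatcher, recoloring the spotlight to the player's light color when IsInside is false.
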(event Custom|DP_MazeGate_Event
  (params (IsInside? :type Boolean))
  (if (not IsInside?)
    (Utilities|FlowControl|Delay 0.0)
    (bind _spotlight (Variables|Default|GetSpotLight)
      (:then
        (Rendering|Components|Light|SetLightColor _spotlight (Variables|/Game/ThirdPerson/Blueprints/BP_ThirdPersonCharacter.BP_ThirdPersonCharacter_C|GetLightColor (Variables|Default|GetPlayer)) true))
      (:else))))

(event EventBeginPlay
  (bind _asbp_third_person_character (Utilities|Casting|CastToBP_ThirdPersonCharacter (Game|GetPlayerCharacter 0)))
  (bind _output_get (Variables|Default|SetPlayer _asbp_third_person_character))
  (EventDispatchers|AssignDPMazeGate _output_get (delegate Custom|DP_MazeGate_Event))
  (if (not (Variables|Default|GetTrap))
    (if (> (Math|Random|RandomIntegerinRange 0 10) 8)
      (ChildActorComponent|SetChildActorClass (Variables|Default|GetChildActor) "/Game/Labs/Lab3/BP_MedKit.BP_MedKit_C")
      (elif (> (Math|Random|RandomIntegerinRange 0 10) 7)
        (ChildActorComponent|SetChildActorClass (Variables|Default|GetChildActor) "/Game/Labs/Lab2/BP_Gold.BP_Gold_C")))))

(event Collision|EventActorBeginOverlap
  (params (OtherActor :type Actor%20Object%20Reference)))

(event EventTick
  (params (DeltaSeconds :type Float%20%28single-precision%29)))

(fn ConstructionScript
  (bind _gridsize (Variables|Default|GetGridSize))
  (bind _childactor (Variables|Default|GetChildActor))
  (LocalVariables|SetWallLength _gridsize)
  (LocalVariables|SetWallThickness (* _gridsize 0.1))
  (Transformation|SetRelativeScale3D (Variables|Default|GetFloor) (Utilities|CubeSizetoScale (Math|Vector|MakeVector (LocalVariables|GetWallLength) (LocalVariables|GetWallLength) (LocalVariables|GetWallThickness))))
  (if (Variables|MazeOptions|GetWestWall)
    (AddComponent|AddStaticMeshComponent false (Math|Transform|MakeTransform "0, 0, 0" "0, 0, 0" (Utilities|CubeSizetoScale (Math|Vector|MakeVector (LocalVariables|GetWallLength) (LocalVariables|GetWallThickness) (Variables|Default|GetWallHeight))))))
  (if (Variables|MazeOptions|GetSouthWall)
    (AddComponent|AddStaticMeshComponent false (Math|Transform|MakeTransform "0, 0, 0" "0, 0, 0" (Utilities|CubeSizetoScale (Math|Vector|MakeVector (LocalVariables|GetWallThickness) (LocalVariables|GetWallLength) (Variables|Default|GetWallHeight))))))
  (if (Variables|MazeOptions|GetEastWall)
    (AddComponent|AddStaticMeshComponent false (Math|Transform|MakeTransform (Math|Vector|MakeVector 0.0 (- (LocalVariables|GetWallLength) (LocalVariables|GetWallThickness)) 0.0) "0, 0, 0" (Utilities|CubeSizetoScale (Math|Vector|MakeVector (LocalVariables|GetWallLength) (LocalVariables|GetWallThickness) (Variables|Default|GetWallHeight))))))
  (if (Variables|MazeOptions|GetNorthWall)
    (AddComponent|AddStaticMeshComponent false (Math|Transform|MakeTransform (Math|Vector|MakeVector (- (LocalVariables|GetWallLength) (LocalVariables|GetWallThickness)) 0.0 0.0) "0, 0, 0" (Utilities|CubeSizetoScale (Math|Vector|MakeVector (LocalVariables|GetWallThickness) (LocalVariables|GetWallLength) (Variables|Default|GetWallHeight))))))
  (if (Variables|MazeOptions|GetCeiling)
    (AddComponent|AddStaticMeshComponent false (Math|Transform|MakeTransform (Math|Vector|MakeVector 0.0 0.0 (Variables|Default|GetWallHeight)) "0, 0, 0" (Utilities|CubeSizetoScale (Math|Vector|MakeVector (LocalVariables|GetWallLength) (LocalVariables|GetWallLength) (LocalVariables|GetWallThickness))))))
  (if (> (Variables|MazeOptions|GetLightIntensity) 0.0)
    (bind _returnvalue (AddComponent|AddSpotLightComponent false (Math|Transform|MakeTransform (Math|Vector|MakeVector (* (LocalVariables|GetWallLength) 0.5) (* (LocalVariables|GetWallLength) 0.5) (- (Variables|Default|GetWallHeight) (LocalVariables|GetWallThickness))) "-90.000000,0.000000,0.000000" "1.000000,1.000000,1.000000")))
    (bind _output_get (Variables|Default|SetSpotLight _returnvalue))
    (Rendering|Components|Light|SetIntensity _output_get (Variables|MazeOptions|GetLightIntensity))
    (Rendering|Components|Light|SetLightColor _output_get (Variables|MazeOptions|GetDefaultLight%20Color) true))
  (Transformation|SetRelativeLocation (Variables|Default|GetScene) (Math|Vector|MakeVector (* (LocalVariables|GetWallLength) 0.5) (* (LocalVariables|GetWallLength) 0.5) (* (LocalVariables|GetWallLength) 0.1)) false false)
  (switch Utilities|FlowControl|Switch|SwitchonEnum_TrapTypes (Variables|Default|GetTrapType)
    (:NewEnumerator0
      (Variables|Default|SetTrap false))
    (:NewEnumerator1
      (Variables|Default|SetTrap true)
      (ChildActorComponent|SetChildActorClass _childactor "/Game/Labs/Lab3/BP_SpikeTrap.BP_SpikeTrap_C"))
    (:NewEnumerator2
      (Variables|Default|SetTrap true)
      (ChildActorComponent|SetChildActorClass _childactor "/Game/Labs/Lab3/BP_AxeTrap.BP_AxeTrap_C")
      (Transformation|SetRelativeRotation _childactor (Variables|Default|GetTrapRotation) false false))
    (:NewEnumerator3
      (Variables|Default|SetTrap true)
      (ChildActorComponent|SetChildActorClass _childactor "/Game/Labs/Lab3/GasTrap.GasTrap_C"))))